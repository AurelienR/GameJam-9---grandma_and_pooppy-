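; Poopy is the Paper2D side-scrolling kaiju hero, auto-advancing along X until touching an EndWall, with axis movement and button or touch jumping.
; Tick faces it along its velocity and picks walk, jump or idle flipbooks by comparing current and previous velocities.
; BeginPlay creates the HUD and sound manager with looping grunts.
; Missile hits hide life icons until the lose level loads; enough peasant deaths trigger rampage once.
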(event `UpdateAnimation`
  (bind (_returnvalue_x _returnvalue_y _returnvalue_z) (`KismetMathLibrary.BreakVector` (`self.GetVelocity`)))
  ;[1 1 1] Handle Animation
  (if (`self.animation en cours`)
    _
    (elif (== (`KismetMathLibrary.VSize` (`self.GetVelocity`)) 0.0)
      (`PaperFlipbookComponent.SetFlipbook` (`self.Sprite`) "/Game/Sprites/PooPy/Idle-flipbook.Idle-flipbook")
      (elif (!= _returnvalue_z 0.0)
        (`self.Saut`)
        (elif (or (!= _returnvalue_x 0.0) (`self.Touchelefond`))
          (`self.Marche`))))))

(event `self.ReceiveBeginPlay`
  ;[1 1 1] Init
  (set `self.Nb_paysans_mort` 0)
  (bind _returnvalue (`|CreateWidget` "/Game/UI/HUD.HUD_C"))
  (bind _output_get (set `self.Hud` _returnvalue))
  (`UserWidget.AddToViewport` _returnvalue 0)
  (`/Game/UI/HUD.Event Display Objective` _output_get)
  (`AudioComponent.Play` (`self.Audio`) 0.0)
  (bind _returnvalue_2 (`|SpawnActorFromClass` "/Game/Sound/SoundAmbientManager.SoundAmbientManager_C" (`KismetMathLibrary.MakeTransform` (0.0 0.0 0.0)) "Undefined" "OverrideRootScale"))
  (set `self.sound_manager` _returnvalue_2)
  (`KismetSystemLibrary.K2_SetTimer` self "grunting" 6.0 true))

(event `grunting`
  (`/Game/Sound/SoundAmbientManager.Event Kayju Grunt` (`self.sound_manager`)))

(event `self.ReceiveTick`
  (params (DeltaSeconds :type "Float (single-precision)"))
  (bind (_returnvalue_x _returnvalue_y _returnvalue_z) (`KismetMathLibrary.BreakVector` (+ (`self.K2_GetActorLocation`) (`KismetMathLibrary.MakeVector` (`self.vitesse_route_poopy`)))))
  ;[1 1 1] Tick - Updates animation
  (`|ExecutionSequence`
    (:`then_0`
      (`self.UpdateAnimation`)
      (`/Engine/EditorBlueprintResources/StandardMacros.CompareFloat` (.x (`MovementComponent.Velocity` (`self.GetMovementComponent`)))
        (:`>`
          (`Controller.SetControlRotation` (`self.GetController`) (`KismetMathLibrary.MakeRotator` 0.0 0.0 0.0)))
        (:`<`
          (`Controller.SetControlRotation` (`self.GetController`) (`KismetMathLibrary.MakeRotator` 0.0 0.0 180.0)))))
    (:`then_1`
      (if (not (`self.Touchelefond`))
        (`self.K2_SetActorLocation` (`KismetMathLibrary.MakeVector` _returnvalue_x 80.0 _returnvalue_z))))
    (:`then_2`
      (if (and (>= (`self.Nb_paysans_mort`) (`self.Nb_mort_avant_rampage`)) (not (`self.Rampage_launched`)))
        (`self.Launch_Rampage`)
        (set `self.Rampage_launched` true)))))

(event `InputAxis|MoveRight`
  (params (AxisValue :type "Float (single-precision)"))
  (bind _returnvalue_x (`KismetMathLibrary.BreakVector` (`self.GetVelocity`)))
  ;[1 1 1] Handle movement
  (if (> _returnvalue_x 0.0)
    (`self.AddMovementInput` (1.0 0.0 0.0) (* AxisValue 5.0))
    (else
      (`self.AddMovementInput` (1.0 0.0 0.0) AxisValue))))

(event `InputAction|Jump`
  (params (Key :type "Key Structure" :default "AnyKey"))
  ;[1 1 1] Handle Jump
  (:`Pressed`
    (set `self.animation en cours` true :!label _label)
    (`PaperFlipbookComponent.SetFlipbook` (`self.Sprite`) "/Game/Sprites/PooPy/saut/Saut-debut-flipbook.Saut-debut-flipbook")
    (`KismetSystemLibrary.Delay` 0.2)
    (set `self.animation en cours` false)
    (`self.Jump`)
    (`/Game/Sound/SoundAmbientManager.Event Kayju Jump` (`self.sound_manager`)))
  (:`Released`
    (`self.StopJumping` :!label _label_2)))

(event `InputTouch`
  (params (Location :type "Vector Structure") (FingerIndex :type "ETouchIndex Enum"))
  ;[1 1 1] Handle Jump
  (:`Pressed`
    (goto _label))
  (:`Released`
    (goto _label_2)))

(event `self.ReceiveActorBeginOverlap`
  (params (OtherActor :type "Actor Object Reference"))
  (bind _returnvalue (- (`self.life point`) 1))
  ;[1 1 1] Gestion peut pas sortir a gauche
  (cast `/Game/Blueprints/Scenes/EndWall` OtherActor
    (:`then`
      (set `self.Touchelefond` true))
    (:`CastFailed`
      (cast `/Game/Blueprints/Scenes/Missiles` OtherActor)
      (`SceneComponent.SetVisibility` (`/Game/Blueprints/LifePoints/LifePoint.PaperFlipbook` (`KismetArrayLibrary.Array_Get` (`self.Life Point Tab`) _returnvalue)) false false)
      (bind _output_get (set `self.life point` _returnvalue))
      (if (<= _output_get 0)
        (`self.Loose`)))))

(event `self.ReceiveActorEndOverlap`
  (params (OtherActor :type "Actor Object Reference"))
  ;[1 1 1] Gestion peut pas sortir a gauche
  (cast `/Game/Blueprints/Scenes/EndWall` OtherActor)
  (set `self.Touchelefond` false))

(event `Launch_Rampage`
  ;[1 1 1] rampage
  (`/Game/UI/HUD.Event Display Rampage` (`self.Hud`))
  (`AudioComponent.SetSound` (`self.Audio`) "/Game/Sound/vener_mode_Cue.vener_mode_Cue"))

(fn `Loose`
  (`Widget.RemoveFromParent` (`self.Hud`))
  (`self.K2_DestroyActor`)
  (`GameplayStatics.OpenLevel` "level-loose")
  (return))

(fn `Marche`
  (bind _returnvalue_x (`KismetMathLibrary.BreakVector` (`self.GetVelocity`)))
  (bind _output_get (set `self.velocity_x` _returnvalue_x))
  (if (and (== (`self.Ancien_velocity_x`) 0.0) (!= _output_get 0.0))
    (`PaperFlipbookComponent.SetFlipbook` (`self.Sprite`) "/Game/Sprites/PooPy/marche-arret/arret-marche-flipbook.arret-marche-flipbook")
    (set `self.Ancien_velocity_x` (`self.velocity_x`) :!label _label)
    (elif (and (!= 0.0 (`self.Ancien_velocity_x`)) (== 0.0 (`self.velocity_x`)))
      (`PaperFlipbookComponent.SetFlipbook` (`self.Sprite`) "/Game/Sprites/PooPy/arret-marche/marche-arret-flipbook.marche-arret-flipbook")
      (goto _label)
      (else
        (`PaperFlipbookComponent.SetFlipbook` (`self.Sprite`) "/Game/Sprites/PooPy/marche/marche-flibook.marche-flibook"))))
  (return))

(fn `Saut`
  (bind (_returnvalue_x _returnvalue_y _returnvalue_z) (`KismetMathLibrary.BreakVector` (`self.GetVelocity`)))
  (bind (_returnvalue_x_2 _returnvalue_y_2 _returnvalue_z_2) (`KismetMathLibrary.BreakVector` (`self.GetVelocity`)))
  (set `self.velocity_z` _returnvalue_z_2)
  (if (and (== 0.0 (`self.Ancien_velocity_z`)) (!= _returnvalue_z_2 0.0))
    (`PaperFlipbookComponent.SetFlipbook` (`self.Sprite`) "/Game/Sprites/PooPy/saut/Saut-debut-flipbook.Saut-debut-flipbook")
    (elif (and (!= 0.0 (`self.Ancien_velocity_z`)) (== 0.0 _returnvalue_z))
      (`PaperFlipbookComponent.SetFlipbook` (`self.Sprite`) "/Game/Sprites/PooPy/saut/saut-atterissage.saut-atterissage")
      (elif (> (`self.velocity_z`) 0.0)
        (`PaperFlipbookComponent.SetFlipbook` (`self.Sprite`) "/Game/Sprites/PooPy/saut/Saut-montee.Saut-montee")
        (else
          (`PaperFlipbookComponent.SetFlipbook` (`self.Sprite`) "/Game/Sprites/PooPy/saut/saut-descente.saut-descente")))))
  (set `self.Ancien_velocity_z` (`self.velocity_z`))
  (return))

(fn `UserConstructionScript`)

(fn `winning_poopy`
  (`Widget.RemoveFromParent` (`self.Hud`))
  (`self.K2_DestroyActor`)
  (`GameplayStatics.OpenLevel` "level2")
  (return))