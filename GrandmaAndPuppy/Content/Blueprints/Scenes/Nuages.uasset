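; Scrolling cloud actor that drifts along negative X and removes itself once it leaves the play area.
; The construction script picks a random speed and adds one of three random cloud sprites.
; BeginPlay and Tick share movement logic that applies a swept, per-frame offset without delta-time scaling.
; Past the X limit, it adds an empty sprite component each pass and destroys itself after a short delay.
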(event `self.ReceiveBeginPlay`
  ;[1 1 1] NuageSpawner
  (if (< (.x (`self.Nuage Location`)) -1600.0) :!label _label
    (bind _returnvalue (`AddComponent|PaperSpriteComponent_3`))
    (`PaperSpriteComponent.SetSprite` _returnvalue null)
    (`KismetSystemLibrary.Delay` 1.0)
    (`self.K2_DestroyActor`)
    (else
      (bind _output_get (set `self.Nuage Location` (+ (`self.K2_GetActorLocation`) (`KismetMathLibrary.MakeVector` (`self.Nuage Speed`)))))
      (`self.K2_SetActorLocation` _output_get true))))

(event `self.ReceiveTick`
  (params (DeltaSeconds :type "Float (single-precision)"))
  ;[1 1 1] NuageSpawner
  (goto _label))

(fn `UserConstructionScript`
  (set `self.Nuage Speed` (`KismetMathLibrary.RandomFloatInRange` -3.0 -7.0))
  (bind _output_get (set `self.Cloud1` "/Game/Sprites/Cloud/cloud1_Sprite_0.cloud1_Sprite_0"))
  (bind _output_get_2 (set `self.Cloud 2` "/Game/Sprites/Cloud/cloud2_Sprite_0.cloud2_Sprite_0"))
  (bind _output_get_3 (set `self.Cloud 3` "/Game/Sprites/Cloud/cloud3_Sprite_0.cloud3_Sprite_0"))
  (bind _returnvalue (`AddComponent|Paper Sprite Component_2`))
  (`PaperSpriteComponent.SetSprite` _returnvalue (`KismetArrayLibrary.Array_Get` (`|MakeArray` _output_get _output_get_2 _output_get_3) (`KismetMathLibrary.RandomIntegerInRange` 0 2))))