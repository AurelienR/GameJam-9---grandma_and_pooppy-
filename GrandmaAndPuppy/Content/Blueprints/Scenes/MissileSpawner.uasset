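; MissileSpawner is an actor that launches a limited series of Missiles actors from its placement in the level.
; On BeginPlay it spawns one immediately at its own transform, with the height randomized upward within a fixed band.
; A DoN node and random Delay loop back to the spawn, producing ten further missiles at irregular intervals before stopping.
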(event `self.ReceiveBeginPlay`
  (bind _z (.z (.location (`self.GetTransform`))))
  (`|SpawnActorFromClass` "/Game/Blueprints/Scenes/Missiles.Missiles_C" (`KismetMathLibrary.MakeTransform` (`KismetMathLibrary.MakeVector` (.x (.location (`self.GetTransform`))) (.y (.location (`self.GetTransform`))) (`KismetMathLibrary.RandomFloatInRange` _z (+ _z 600.0))) (.rotation (`self.GetTransform`)) (.scale (`self.GetTransform`))) "Undefined" "OverrideRootScale" :!label _label)
  (`/Engine/EditorBlueprintResources/StandardMacros.Do N` 10
    (:`Exit`
      (`KismetSystemLibrary.Delay` (`KismetMathLibrary.RandomFloatInRange` 1.0 5.0))
      (goto _label))))

(event `self.ReceiveActorBeginOverlap`
  (params (OtherActor :type "Actor Object Reference")))

(event `self.ReceiveTick`
  (params (DeltaSeconds :type "Float (single-precision)")))

(fn `UserConstructionScript`)