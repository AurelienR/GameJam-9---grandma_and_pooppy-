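; Poste is a scrolling Paper2D scene actor that serves as a win trigger for the Poopy player character.
; Each tick it shifts a stored position along X by VitesseRoutePoste at a fixed height, without delta-time scaling, and destroys itself past a negative X limit.
; On overlap with a Poopy, it switches its flipbook to Victoire and calls WinningPoopy on the player character.
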(event `self.ReceiveBeginPlay`)

(event `self.ReceiveTick`
  (params (DeltaSeconds :type "Float (single-precision)"))
  (bind _position_x (`KismetMathLibrary.BreakVector` (`self.Position`)))
  (bind (_returnvalue_x _returnvalue_y) (`KismetMathLibrary.BreakVector` (+ (`self.Position`) (`KismetMathLibrary.MakeVector` (`self.Vitesse route poste`) 0.0 150.0))))
  (if (< _position_x -1600.0)
    (`self.K2_DestroyActor`)
    (else
      (bind _output_get (set `self.Position` (`KismetMathLibrary.MakeVector` _returnvalue_x _returnvalue_y 150.0)))
      (`self.K2_SetActorLocation` _output_get))))

(event `self.ReceiveActorBeginOverlap`
  (params (OtherActor :type "Actor Object Reference"))
  (cast `/Game/Blueprints/Heros/Poopy` OtherActor)
  (`PaperFlipbookComponent.SetFlipbook` (`self.PaperFlipbook`) "/Game/Sprites/Poste/victoire.victoire")
  (bind _aspoopy (cast `/Game/Blueprints/Heros/Poopy` (`GameplayStatics.GetPlayerCharacter` 0)))
  (`/Game/Blueprints/Heros/Poopy.winning_poopy` _aspoopy))

(fn `UserConstructionScript`)