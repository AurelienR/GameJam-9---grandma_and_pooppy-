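; Scrolling building actor that Poopy can land on, with an ice cream vendor sprite swap.
; Each Tick it shifts along X at the building road speed from its construction-time position, destroying itself past a negative X limit.
; When Poopy's ground collider enters Boite_haute, Box turns blocking, the sprite changes and Poopy's road speed drops to zero.
; End overlap makes Box ignore collisions and restores Poopy's speed from OldVitesseRoute.
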(event `self.ReceiveBeginPlay`)

(event `self.ReceiveActorBeginOverlap`
  (params (OtherActor :type "Actor Object Reference")))

(event `self.ReceiveTick`
  (params (DeltaSeconds :type "Float (single-precision)"))
  (bind _postion_x (`KismetMathLibrary.BreakVector` (`self.postion`)))
  ;[1 1 1] Deplacement Building
  (if (< _postion_x -1600.0)
    (`self.K2_DestroyActor`)
    (else
      (bind _output_get (set `self.postion` (+ (`self.postion`) (`KismetMathLibrary.MakeVector` (`self.Vitesse_route_buildings`)))))
      (`self.K2_SetActorLocation` _output_get))))

(event `self.boite_haute.OnComponentBeginOverlap`
  (params (OtherActor :type "Actor Object Reference") (OtherComp :type "PrimitiveComponent Object Reference") (OtherBodyIndex :type Integer) (bFromSweep :type Boolean) (SweepResult :type "HitResult Structure (by ref)"))
  (if (not (`self.is_overlapping`))
    (bind _aspoopy (cast `/Game/Blueprints/Heros/Poopy` OtherActor))
    (if (== (`/Game/Blueprints/Heros/Poopy.colision_sol` _aspoopy) OtherComp)
      (`PrimitiveComponent.SetCollisionResponseToAllChannels` (`self.Box`) "ECR_Block")
      (`PaperSpriteComponent.SetSprite` (`self.PaperSprite`) "/Game/Sprites/Marchant_de_glace/marchand_de_glace2_Sprite.marchand_de_glace2_Sprite")
      (set `/Game/Blueprints/Heros/Poopy.vitesse_route_poopy` 0.0 _aspoopy)
      (set `self.is_overlapping` true))))

(event `self.boite_haute.OnComponentEndOverlap`
  (params (OtherActor :type "Actor Object Reference") (OtherComp :type "PrimitiveComponent Object Reference") (OtherBodyIndex :type Integer))
  (if (`self.is_overlapping`)
    (bind _aspoopy (cast `/Game/Blueprints/Heros/Poopy` OtherActor))
    (`PrimitiveComponent.SetCollisionResponseToAllChannels` (`self.Box`) "ECR_Ignore")
    (set `/Game/Blueprints/Heros/Poopy.vitesse_route_poopy` (`self.old_vitesse_route`) _aspoopy)
    (set `self.is_overlapping` false)))

(fn `UserConstructionScript`
  (set `self.postion` (`self.K2_GetActorLocation`)))