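; Side-scrolling background actor that loops the scenery, spawns street content and drives the score of the Poopy player.
; Tick moves two backdrop layers and the road by fixed per-frame steps for parallax, snapping each back after its period.
; Road movement adds to the score pushed to Poopy.
; Self-rearming random timers spawn buildings and staggered groups of civilians off to the side, passing them the road speed.
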(event `self.ReceiveBeginPlay`
  ;[1 1 1] Init
  ;;[1 1 1] init ciel
  (set `self.Score_total` 0)
  (bind _output_get (set `self.Position_initiale_ciel` (`SceneComponent.K2_GetComponentLocation` (`self.Fond_devant`))))
  (bind _output_get_2 (set `self.Position_ciel` _output_get))
  (set `self.x_limite_ciel` (- (.x _output_get_2) (`self.Taille_periode_ciel`)))
  ;;[1 1 1] init route
  (bind _output_get_3 (set `self.Position_initiale_route` (`SceneComponent.K2_GetComponentLocation` (`self.Route`))))
  (bind _output_get_4 (set `self.position_route` _output_get_3))
  (set `self.x_limite_route` (- (.x _output_get_4) (`self.Periode_route`)))
  ;;[1 1 1] init fond2
  (bind _output_get_5 (set `self.Position_initiale_fond2` (`SceneComponent.K2_GetComponentLocation` (`self.Fond_milieu`))))
  (bind _output_get_6 (set `self.Position_fond2` _output_get_5))
  (set `self.X_limite_fond_2` (- (.x _output_get_6) 3060.0))
  (cast `/Game/Blueprints/Heros/Poopy` (`GameplayStatics.GetPlayerCharacter` 0))
  (bind _output_get_7 (set `self.Vitesse_route` -5.0))
  (bind _aspoopy (cast `/Game/Blueprints/Heros/Poopy` (`GameplayStatics.GetPlayerCharacter` 0)))
  (set `/Game/Blueprints/Heros/Poopy.vitesse_route_poopy` _output_get_7 _aspoopy)
  (`KismetSystemLibrary.K2_SetTimer` null "Spawn_immeuble" (`KismetMathLibrary.RandomFloatInRange` (`self.Min_Spawn_building`) (`self.Max_spawn_Buildings`)))
  (`KismetSystemLibrary.K2_SetTimer` null "Spawn_Civils" (`KismetMathLibrary.RandomFloatInRange` (`self.Min_Spawn_Civils`) (`self.Max_spawn_Civils`)))
  (`KismetSystemLibrary.K2_SetTimer` null "" 2.0))

(event `self.ReceiveActorBeginOverlap`
  (params (OtherActor :type "Actor Object Reference")))

(event `self.ReceiveTick`
  (params (DeltaSeconds :type "Float (single-precision)"))
  ;[1 1 1] chaque tick
  ;;[1 1 1] Defiliement ciel
  (`|ExecutionSequence`
    (:`then_0`
      (if (< (.x (`self.Position_ciel`)) (`self.x_limite_ciel`))
        (set `self.Position_ciel` (`self.Position_initiale_ciel`))
        (else
          (set `self.Position_ciel` (+ (`self.Position_ciel`) (-5.0 0.0 0.0)))))
      (`SceneComponent.K2_SetWorldLocation` (`self.Fond_devant`) (`self.Position_ciel`) false false))
    (:`then_1`
      ;[1 1 1] fond 2
      (if (< (.x (`self.Position_fond2`)) (`self.X_limite_fond_2`))
        (set `self.Position_fond2` (`self.Position_initiale_fond2`))
        (else
          (set `self.Position_fond2` (+ (`self.Position_fond2`) (-3.0 0.0 0.0)))))
      (`SceneComponent.K2_SetWorldLocation` (`self.Fond_milieu`) (`self.Position_fond2`) false false))
    (:`then_2`
      ;;[1 1 1] Defilement route
      (if (< (.x (`self.position_route`)) (`self.x_limite_route`))
        (set `self.position_route` (`self.Position_initiale_route`))
        (else
          (bind _output_get (set `self.Score_total` (`KismetMathLibrary.Round` (+ (`KismetMathLibrary.Conv_IntToDouble` (`self.Score_total`)) (- 0.0 (`self.Vitesse_route`))))))
          (bind _aspoopy (cast `/Game/Blueprints/Heros/Poopy` (`GameplayStatics.GetPlayerCharacter` 0)))
          (set `/Game/Blueprints/Heros/Poopy.Score` _output_get _aspoopy)
          (set `self.position_route` (+ (`self.position_route`) (`KismetMathLibrary.MakeVector` (`self.Vitesse_route`))))))
      (`SceneComponent.K2_SetWorldLocation` (`self.Route`) (`self.position_route`) false false))))

(event `Spawn_immeuble`
  ;[1 1 1] Spawn buildings
  (bind _output_get (set `self.Spawn_transform` (`KismetMathLibrary.MakeTransform` (+ (1800.0 100.0 0.0) (.location (`SceneComponent.GetRelativeTransform` (`self.DefaultSceneRoot`)))) (.rotation (`SceneComponent.GetRelativeTransform` (`self.DefaultSceneRoot`))) (.scale (`SceneComponent.GetRelativeTransform` (`self.DefaultSceneRoot`))))))
  (bind _returnvalue (`|SpawnActorFromClass` "/Game/Blueprints/Scenes/Building.Building_C" _output_get "Undefined" "OverrideRootScale"))
  (set `/Game/Blueprints/Scenes/Building.Vitesse_route_buildings` (`self.Vitesse_route`) _returnvalue)
  (set `/Game/Blueprints/Scenes/Building.old_vitesse_route` 0.0 _returnvalue)
  (`KismetSystemLibrary.K2_SetTimer` null "Spawn_immeuble" (`KismetMathLibrary.RandomFloatInRange` (`self.Min_Spawn_building`) (`self.Max_spawn_Buildings`))))

(event `Spawn_Civils`
  (bind _vitesse_route (`self.Vitesse_route`))
  ;[1 1 1] Swpan Civils
  (bind _output_get (set `self.Spawn_transform` (`KismetMathLibrary.MakeTransform` (+ (1600.0 40.0 -150.0) (.location (`SceneComponent.GetRelativeTransform` (`self.DefaultSceneRoot`)))) (.rotation (`SceneComponent.GetRelativeTransform` (`self.DefaultSceneRoot`))) (.scale (`SceneComponent.GetRelativeTransform` (`self.DefaultSceneRoot`))))))
  (for _ (range 1 (+ (`KismetMathLibrary.RandomIntegerInRange` 5 10) 1))
    (bind _returnvalue (`|SpawnActorFromClass` "/Game/Blueprints/Scenes/Civils.Civils_C" _output_get "Undefined" "OverrideRootScale"))
    (set `/Game/Blueprints/Scenes/Civils.Civil_Speed` (+ _vitesse_route -1.0) _returnvalue)
    (set `/Game/Blueprints/Scenes/Civils.Route_speed` _vitesse_route _returnvalue)
    (`KismetSystemLibrary.Delay` 0.1))
  (`KismetSystemLibrary.K2_SetTimer` null "Spawn_Civils" (`KismetMathLibrary.RandomFloatInRange` (`self.Min_Spawn_Civils`) (`self.Max_spawn_Civils`))))

(fn `UserConstructionScript`)