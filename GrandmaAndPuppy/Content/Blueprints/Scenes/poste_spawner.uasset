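; Spawner actor that places a single Poste in the scene once the player's Poopy score exceeds the PosteScore threshold.
; From BeginPlay, a looping random Delay of a few seconds repeatedly polls the score on the player character.
; The Poste spawns at the root component's transform and receives that position and a fixed negative road speed (VitesseRoutePoste).
; The Alreadyposte flag prevents further spawns, though the loop keeps running.
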(event `self.ReceiveBeginPlay`
  (bind _returnvalue (`SceneComponent.GetRelativeTransform` (`self.DefaultSceneRoot`)))
  (bind _aspoopy (cast `/Game/Blueprints/Heros/Poopy` (`GameplayStatics.GetPlayerCharacter` 0)))
  (if (and (> (`/Game/Blueprints/Heros/Poopy.Score` _aspoopy) (`self.Poste score`)) (not (`self.Alreadyposte`))) :!label _label
    (bind _returnvalue_2 (`|SpawnActorFromClass` "/Game/Blueprints/Scenes/Poste.Poste_C" _returnvalue "Undefined" "OverrideRootScale"))
    (set `/Game/Blueprints/Scenes/Poste.Position` (.location _returnvalue) _returnvalue_2)
    (set `/Game/Blueprints/Scenes/Poste.Vitesse route poste` -5.0 _returnvalue_2)
    (set `self.Alreadyposte` true))
  (`KismetSystemLibrary.Delay` (`KismetMathLibrary.RandomFloatInRange` 2.0 7.0))
  (goto _label))

(event `self.ReceiveBeginPlay`)

(event `self.ReceiveActorBeginOverlap`
  (params (OtherActor :type "Actor Object Reference")))

(event `self.ReceiveTick`
  (params (DeltaSeconds :type "Float (single-precision)")))

(fn `UserConstructionScript`)