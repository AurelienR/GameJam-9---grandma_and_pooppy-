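; Missile actor that flies along the X axis and explodes on contact with the player character.
; BeginPlay and every Tick share one movement step that adds RocketSpeed with sweep, without delta-time scaling, and destroys the actor once its stored X drops below a fixed limit.
; Overlapping the player swaps its flipbook to an explosion, then destroys it after a short delay.
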(event `self.ReceiveBeginPlay`
  (bind _rocket_location_x (`KismetMathLibrary.BreakVector` (`self.Rocket Location`)))
  ;[1 1 1] MissilMovment
  (if (< _rocket_location_x -1600.0) :!label _label
    (`self.K2_DestroyActor`)
    (else
      (bind _output_get (set `self.Rocket Location` (+ (`self.K2_GetActorLocation`) (`KismetMathLibrary.MakeVector` (`self.Rocket Speed`)))))
      (`self.K2_SetActorLocation` _output_get true))))

(event `self.ReceiveTick`
  (params (DeltaSeconds :type "Float (single-precision)"))
  ;[1 1 1] MissilMovment
  (goto _label))

(event `self.ReceiveActorBeginOverlap`
  (params (OtherActor :type "Actor Object Reference"))
  ;[1 1 1] CharacterCollision
  (if (== OtherActor (`GameplayStatics.GetPlayerCharacter` 0))
    (`PaperFlipbookComponent.SetFlipbook` (`self.missile_flipbook`) "/Game/Sprites/Missiles/explosion/explo-flipbook.explo-flipbook")
    (`KismetSystemLibrary.Delay` 0.2)
    (`self.K2_DestroyActor`)))

(fn `UserConstructionScript`)