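; Scene actor that continuously spawns Nuages (cloud) actors above itself from BeginPlay onward.
; Each spawn keeps the spawner's rotation, sits at a random height in a band above it with a tiny Y jitter, and gets a randomized per-axis scale offset.
; A randomized Delay of a few seconds loops back to the spawn, so the spawning repeats without end and without using Tick.
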(event `self.ReceiveBeginPlay`
  (bind _returnvalue (`KismetMathLibrary.RandomFloatInRange` -0.7 0.2))
  (bind _returnvalue_2 (+ (.z (.location (`self.GetTransform`))) 500.0))
  (`|SpawnActorFromClass` "/Game/Blueprints/Scenes/Nuages.Nuages_C" (`KismetMathLibrary.MakeTransform` (`KismetMathLibrary.MakeVector` (.x (.location (`self.GetTransform`))) (+ (.y (.location (`self.GetTransform`))) (`KismetMathLibrary.RandomFloatInRange` 0.0 1.0)) (`KismetMathLibrary.RandomFloatInRange` _returnvalue_2 (+ _returnvalue_2 300.0))) (.rotation (`self.GetTransform`)) (+ (.scale (`self.GetTransform`)) (`KismetMathLibrary.MakeVector` _returnvalue _returnvalue _returnvalue))) "Undefined" "OverrideRootScale" :!label _label)
  (`KismetSystemLibrary.Delay` (`KismetMathLibrary.RandomFloatInRange` 2.0 7.0))
  (goto _label))

(event `self.ReceiveActorBeginOverlap`
  (params (OtherActor :type "Actor Object Reference")))

(event `self.ReceiveTick`
  (params (DeltaSeconds :type "Float (single-precision)")))

(fn `UserConstructionScript`)