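; Civilian (peasant) actor that moves along X until it is hit by the Poopy character or leaves the scene.
; Each tick it offsets its cached location by CivilSpeed and destroys itself once X drops below -1600.
; On first overlap with Poopy, it switches to RouteSpeed and a splat flipbook, ignores collisions, increments Poopy's peasant death count and fires the death event on the player's SoundManager.
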(event `self.ReceiveBeginPlay`)

(event `self.ReceiveTick`
  (params (DeltaSeconds :type "Float (single-precision)"))
  (bind _civil_location_x (`KismetMathLibrary.BreakVector` (`self.Civil_location`)))
  ;[1 1 1] Deplacement du paysans
  (if (< _civil_location_x -1600.0)
    (`self.K2_DestroyActor`)
    (else
      (bind _output_get (set `self.Civil_location` (+ (`self.Civil_location`) (`KismetMathLibrary.MakeVector` (`self.Civil_Speed`)))))
      (`self.K2_SetActorLocation` _output_get))))

(event `self.ReceiveActorBeginOverlap`
  (params (OtherActor :type "Actor Object Reference"))
  ;[1 1 1] Collision avec Poopy
  (if (not (`self.isplaying`))
    (bind _aspoopy (cast `/Game/Blueprints/Heros/Poopy` OtherActor))
    (set `self.isplaying` true)
    (set `self.Civil_Speed` (`self.Route_speed`))
    (set `/Game/Blueprints/Heros/Poopy.Nb_paysans_mort` (+ (`/Game/Blueprints/Heros/Poopy.Nb_paysans_mort` _aspoopy) 1) _aspoopy)
    (`PaperFlipbookComponent.SetFlipbook` (`self.PaperFlipbook`) "/Game/Sprites/Paysans/SploutchFlipbook.SploutchFlipbook")
    (`PrimitiveComponent.SetCollisionResponseToAllChannels` (`self.CollisionBox`) "ECR_Ignore")
    (bind _aspoopy_2 (cast `/Game/Blueprints/Heros/Poopy` (`GameplayStatics.GetPlayerCharacter` 0)))
    (`/Game/Sound/SoundAmbientManager.Event Civil Death` (`/Game/Blueprints/Heros/Poopy.sound_manager` _aspoopy_2))))

(fn `UserConstructionScript`
  (set `self.Civil_location` (`self.K2_GetActorLocation`)))